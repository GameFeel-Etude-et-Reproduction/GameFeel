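; Windmill actor that spins its palms (blades) mesh around the pitch axis when play begins.
; A start-up timeline drives the first turn, then a second timeline repeats full turns until a counter reaches its limit.
; A final stop timeline then runs, but its lerp alpha is fixed at zero, so it holds the blades at zero pitch.
; The WindIson event and Interact function are empty.
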(event `/Game/BenoitTest/BPI_MagicInterface.WindIsOn`)

(event `self.ReceiveBeginPlay`
  (bind (_direction _startrotating) (`Timeline|InitiateRotation` :!via `PlayFromStart`)
    (:`Update`
      (`SceneComponent.K2_SetRelativeRotation` (`self.SM_WindMill_Palms`) (`KismetMathLibrary.MakeRotator` 0.0 (`KismetMathLibrary.Lerp` 0.0 360.0 _startrotating)) false false))
    (:`Finished`
      (bind (_direction_2 _newtrack_1) (`Timeline|rot` :!label _label)
        (:`Update`
          (`SceneComponent.K2_SetRelativeRotation` (`self.SM_WindMill_Palms`) (`KismetMathLibrary.MakeRotator` 0.0 (`KismetMathLibrary.Lerp` 0.0 359.0 _newtrack_1)) false false))
        (:`Finished`
          (if (!= (`self.compteur`) 2)
            (`self.replay`)
            (set `self.compteur` (+ (`self.compteur`) 1))
            (else
              (`Timeline|StopRo`
                (:`Update`
                  (`SceneComponent.K2_SetRelativeRotation` (`self.SM_WindMill_Palms`) (`KismetMathLibrary.MakeRotator` 0.0 (`KismetMathLibrary.Lerp` 0.0 359.0)) false false))))))))))

(event `replay`
  (goto _label :!via `PlayFromStart`))

(fn `Interact`
  (returns (`Static Mesh` :type "StaticMesh Object Reference"))
  (return null))

(fn `UserConstructionScript`)