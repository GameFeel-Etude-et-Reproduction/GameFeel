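; BP_enigmeManager is a puzzle manager that switches on a windmill's wind when its altar puzzle is judged solved.
; Its verif event loops over ListeAutel, casting each altar to BP_Enigma_Receiver and copying its ItemValid state into EnigmeReussi.
; Each iteration overwrites that flag, so only the last altar decides whether WindIsOnMessage is sent to Windmill.
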(event `verif`
  (for _array_element (`self.listeAutel`)
    (if (`/Game/Ajout_Custom/adrian/BP_Enigma_Receiver.bItemValid` (cast `/Game/Ajout_Custom/adrian/BP_Enigma_Receiver` _array_element :!pure true))
      (set `self.enigmeReussi` true)
      (else
        (set `self.enigmeReussi` false))))
  (if (`self.enigmeReussi`)
    (message `/Game/BenoitTest/BPI_MagicInterface.WindIsOn` (`self.windmill`))))

(fn `UserConstructionScript`)