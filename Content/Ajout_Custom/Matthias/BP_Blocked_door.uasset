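; BP_Blocked_door is a one-shot trigger door that rotates when the player enters its box, then blacks out the screen.
; The box overlap passes through a DoOnce and plays a Timeline, used only as a ticker with Delays on its update.
; Each delayed step adds a small relative rotation to the door.
; A longer delay leads to a near-instant, held camera fade for BP_FirstPersonCharacter.
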(event `self.Box.OnComponentBeginOverlap`
  (params (OverlappedComponent :type "PrimitiveComponent Object Reference") (OtherActor :type "Actor Object Reference") (OtherComp :type "PrimitiveComponent Object Reference") (OtherBodyIndex :type Integer) (bFromSweep :type Boolean) (SweepResult :type "HitResult Structure (by ref)"))
  (if (== OtherActor (`GameplayStatics.GetPlayerPawn` 0))
    (`/Engine/EditorBlueprintResources/StandardMacros.DoOnce` false
      (:`Completed`
        (`Timeline|Timeline`
          (:`Update`
            (`|ExecutionSequence`
              (:`then_0`
                (`KismetSystemLibrary.Delay` 0.01)
                (`SceneComponent.K2_AddRelativeRotation` (`self.Door`) (struct :`Yaw` 0.5) false false))
              (:`then_1`
                (`KismetSystemLibrary.Delay` 0.4)
                (cast `/Game/FirstPerson/Blueprints/BP_FirstPersonCharacter` OtherActor)
                (`PlayerCameraManager.StartCameraFade` :`self` (`GameplayStatics.GetPlayerCameraManager` 0) :`ToAlpha` 1.0 :`Duration` 1e-05 :`bHoldWhenFinished` true)))))))))

(fn `UserConstructionScript`)