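; MBP_Item is a pickup item Blueprint that hands its static mesh to the first-person player when interacted with.
; Interact triggers the Destroy event and returns the mesh to the caller.
; Destroy casts player pawn 0 to BP_FirstPersonCharacter, passes the mesh to TakeObject, then destroys the actor after a brief delay.
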(event `Destroy`
  (`/Game/FirstPerson/Blueprints/BP_FirstPersonCharacter.takeObject` (cast `/Game/FirstPerson/Blueprints/BP_FirstPersonCharacter` (`GameplayStatics.GetPlayerPawn` 0) :!pure true) (`StaticMeshComponent.StaticMesh` (`self.StaticMesh`)))
  (`KismetSystemLibrary.Delay` 0.05)
  (`self.K2_DestroyActor`))

(fn `Interact`
  (returns (`Static Mesh` :type "StaticMesh Object Reference"))
  (`self.Destroy`)
  (return (`StaticMeshComponent.StaticMesh` (`self.StaticMesh`))))

(fn `UserConstructionScript`)