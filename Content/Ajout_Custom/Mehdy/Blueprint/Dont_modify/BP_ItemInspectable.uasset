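; BP_ItemInspectable is an item actor the player can pull up in front of the first-person camera to inspect, then send back to its original place.
; On BeginPlay it caches its transform.
; Inspect flags BP_FirstPersonCharacter as inspecting, calls its InspectObject, and a timeline lerps the item's location to a point just ahead of the camera.
; stopInspecting halts that timeline and starts another that blends the actor back to the cached transform.
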(event `self.ReceiveBeginPlay`
  (set `self.PreviousTransform` (`self.GetTransform`)))

(event `/Game/Ajout_Custom/Mehdy/Blueprint/Dont_modify/BPI_Interact.Inspect`
  (bind _previoustransform_location (`KismetMathLibrary.BreakTransform` (`self.PreviousTransform`)))
  (bind _asbp_first_person_character (cast `/Game/FirstPerson/Blueprints/BP_FirstPersonCharacter` (`GameplayStatics.GetPlayerPawn` 0)))
  (set `/Game/FirstPerson/Blueprints/BP_FirstPersonCharacter.isInspecting` true _asbp_first_person_character)
  (`/Game/FirstPerson/Blueprints/BP_FirstPersonCharacter.inspectObject` _asbp_first_person_character null)
  (bind (_direction _newtrack_0) (`Timeline|Timeline` :!via `PlayFromStart` :!label _label)
    (:`Update`
      (bind _firstpersoncamera (`/Game/FirstPerson/Blueprints/BP_FirstPersonCharacter.FirstPersonCamera` _asbp_first_person_character))
      (`self.K2_SetActorLocation` (`KismetMathLibrary.VLerp` _previoustransform_location (+ (`SceneComponent.K2_GetComponentLocation` _firstpersoncamera) (* (`SceneComponent.GetForwardVector` _firstpersoncamera) 100.0)) _newtrack_0)))))

(event `stopInspecting`
  (`|ExecutionSequence`
    (:`then_0`
      (goto _label :!via `Stop`))
    (:`then_1`
      (bind (_direction _newtrack_0) (`Timeline|Timeline_0` :!via `PlayFromStart`)
        (:`Update`
          (`self.K2_SetActorTransform` (`KismetMathLibrary.TLerp` (`self.GetTransform`) (`self.PreviousTransform`) _newtrack_0)))))))

(fn `UserConstructionScript`
  (`parent.UserConstructionScript`))