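; Inspectable object actor that flies up in front of the first-person camera for inspection and returns to its resting place afterwards.
; Inspect flags the player character as inspecting, hands itself to it, then a timeline lerps its location to 100 units ahead of the camera.
; stopInspecting uses a second timeline to blend the current transform back to the one saved at BeginPlay.
; Interact is an empty stub.
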(event `self.ReceiveBeginPlay`
  (set `self.original position` (`self.GetTransform`)))

(event `/Game/Ajout_Custom/Mehdy/Blueprint/Dont_modify/BPI_Interact.Inspect`
  (bind _original_position_location (`KismetMathLibrary.BreakTransform` (`self.original position`)))
  (bind _asbp_first_person_character (cast `/Game/FirstPerson/Blueprints/BP_FirstPersonCharacter` (`GameplayStatics.GetPlayerPawn` 0) :!pure true))
  (bind _firstpersoncamera (`/Game/FirstPerson/Blueprints/BP_FirstPersonCharacter.FirstPersonCamera` _asbp_first_person_character))
  (set `/Game/FirstPerson/Blueprints/BP_FirstPersonCharacter.isInspecting` true _asbp_first_person_character)
  (`/Game/FirstPerson/Blueprints/BP_FirstPersonCharacter.inspectObject` _asbp_first_person_character self)
  (bind (_direction _newtrack_0) (`Timeline|Timeline` :!via `PlayFromStart`)
    (:`Update`
      (`self.K2_SetActorLocation` (`KismetMathLibrary.VLerp` _original_position_location (+ (`SceneComponent.K2_GetComponentLocation` _firstpersoncamera) (* (`SceneComponent.GetForwardVector` _firstpersoncamera) 100.0)) _newtrack_0)))))

(event `stopInspecting`
  (bind (_direction _newtrack_0) (`Timeline|Timeline_0` :!via `PlayFromStart`)
    (:`Update`
      (`self.K2_SetActorTransform` (`KismetMathLibrary.TLerp` (`self.GetTransform`) (`self.original position`) _newtrack_0)))))

(fn `Interact`
  (returns (`Static Mesh` :type "StaticMesh Object Reference"))
  (return null))

(fn `UserConstructionScript`)